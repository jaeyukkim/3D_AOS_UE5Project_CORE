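; Gameplay Ability for Kwang's RMB attack, dealing area damage to living non-friendly players.
; It picks a sword or no-sword montage from Kwang's active-weapon flag and waits for the Combat.Attack gameplay event.
; That event triggers a radius check around Kwang, or around the sword's location with a particle burst when the weapon is inactive.
; The ability ends when the montage completes, blends out or is interrupted.
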(event Ability|EventActivateAbility
  (bind _returnvalue (Ability|GetAvatarActorfromActorInfo))
  (Class|GameplayAbilityBase|ActivateCasting)
  (Ability|CommitAbility)
  (Utilities|IsValid _returnvalue
    (:Is%20Valid
      (bind _askwang_player (Utilities|Casting|CastToKwangPlayer _returnvalue))
      (Utilities|IsValid _askwang_player
        (:Is%20Valid
          (bind _output_get (Variables|Default|SetKwang _askwang_player))
          (bind _returnvalue_2 (Class|KwangPlayer|GetbActiveWep _output_get))
          (if _returnvalue_2
            (|PlayMontageandWaitProxy "None" "/Game/BP/Character/Kwang/Animation/Ability_RMB_Montage.Ability_RMB_Montage" 1.0 "None" false 1.0 0.0 false
              (:then
                (Ability|Tasks|WaitGameplayEvent "(TagName=\"Abilities.Combat.Attack\")" 0
                  (:EventReceived
                    (Variables|Default|SetAttackLocation (Transformation|GetActorLocation (Ability|GetAvatarActorfromActorInfo)))
                    (CallFunction|ApplingAttack :!label _label))))
              (:OnCompleted
                (Ability|EndAbility :!label _label_2))
              (:OnBlendOut
                (goto _label_2))
              (:OnInterrupted
                (goto _label_2))
              (:OnCancelled
                (goto _label_2)))
            (else
              (|PlayMontageandWaitProxy "None" "/Game/BP/Character/Kwang/Animation/Ability_RMB_NoSword_Montage.Ability_RMB_NoSword_Montage" 1.0 "None" false 1.0 0.0 false
                (:then
                  (bind _returnvalue_3 (Class|KwangPlayer|GetSwordLocation (Variables|Default|GetKwang)))
                  (Variables|Default|SetAttackLocation _returnvalue_3)
                  (Ability|Tasks|WaitGameplayEvent "(TagName=\"Abilities.Combat.Attack\")" 0
                    (:EventReceived
                      (Class|GameplayAbilityBase|SpawnParticleatLocation (Variables|Default|GetAttackLocation) (Variables|Default|GetAttackParticle))
                      (goto _label))))
                (:OnCompleted
                  _)
                (:OnBlendOut
                  _)
                (:OnInterrupted
                  _)
                (:OnCancelled
                  _))
              (Ability|EndAbility))))))))

(event Ability|EventOnEndAbility
  (params (bWasCancelled :type Boolean)))

(fn ApplingAttack
  (bind _returnvalue (Ability|GetAvatarActorfromActorInfo))
  (bind _outoverlappingactors (Class|BlueprintFunctionLibraryBase|GetLivePlayersWithinRadius _returnvalue (Utilities|Array|MakeArray _returnvalue) (Variables|Default|GetAttackRadius) (Variables|Default|GetAttackLocation)))
  (for _array_element _outoverlappingactors
    (Utilities|IsValid _array_element
      (:Is%20Valid
        (bind _returnvalue_2 (Class|BlueprintFunctionLibraryBase|IsFriends _array_element (Ability|GetAvatarActorfromActorInfo)))
        (if (not _returnvalue_2)
          (Class|DamageGameplayAbilityBase|CauseDamage _array_element))))))