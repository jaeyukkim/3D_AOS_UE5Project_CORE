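; Gameplay ability for Kwang's R skill when he has no active weapon: he teleports to his sword and attacks around it.
; It ends early if the weapon is active; otherwise it commits and plays a montage whose gameplay events drive the sequence.
; On authority, the first event moves Kwang to the sword, destroys it and re-arms him.
; A following attack event damages non-friendly live players within a radius of that location.
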(event Ability|EventActivateAbility
  (bind _returnvalue (Ability|GetAvatarActorfromActorInfo))
  (Utilities|IsValid _returnvalue
    (:Is%20Valid
      (bind _askwang_player (Utilities|Casting|CastToKwangPlayer _returnvalue)
        (:then
          (Utilities|IsValid _askwang_player
            (:Is%20Valid
              (bind _output_get (Variables|Default|SetKwang _askwang_player))
              (bind _returnvalue_2 (Class|KwangPlayer|GetbActiveWep _output_get))
              (if _returnvalue_2
                (Ability|EndAbility :!label _label)
                (else
                  (Class|GameplayAbilityBase|ActivateCasting)
                  (Ability|CommitAbility)
                  (|PlayMontageandWaitProxy "None" "/Game/BP/Character/Kwang/Animation/Ability_R_NoWep_Montage.Ability_R_NoWep_Montage" 1.0 "None" false 1.0 0.0 false
                    (:then
                      (Ability|Tasks|WaitGameplayEvent "(TagName=\"Montage.Kwang\")" 0
                        (:EventReceived
                          (Ability|HasAuthority
                            (:True
                              (bind _returnvalue_3 (Class|KwangPlayer|GetSwordLocation (Variables|Default|GetKwang)))
                              (bind _output_get_2 (Variables|Default|SetAttackLotation _returnvalue_3))
                              (Transformation|SetActorLocation (Ability|GetAvatarActorfromActorInfo) _output_get_2 false false)
                              (Class|KwangPlayer|DestroySword (Variables|Default|GetKwang))
                              (Class|KwangPlayer|SetbActiveWep (Variables|Default|GetKwang) true))
                            (:False
                              _))
                          (Ability|Tasks|WaitGameplayEvent "(TagName=\"Abilities.Combat.Attack\")" 0
                            (:EventReceived
                              (CallFunction|ApplingAttack))))))
                    (:OnCompleted
                      (Ability|EndAbility :!label _label_2))
                    (:OnBlendOut
                      (goto _label_2))
                    (:OnInterrupted
                      (goto _label_2))
                    (:OnCancelled
                      (goto _label_2))))))
            (:Is%20Not%20Valid
              (goto _label))))
        (:CastFailed
          (goto _label))))))

(event Ability|EventOnEndAbility
  (params (bWasCancelled :type Boolean)))

(fn ApplingAttack
  (bind _returnvalue (Ability|GetAvatarActorfromActorInfo))
  (bind _outoverlappingactors (Class|BlueprintFunctionLibraryBase|GetLivePlayersWithinRadius _returnvalue (Utilities|Array|MakeArray _returnvalue) (Variables|Default|GetAttackRadius) (Variables|Default|GetAttackLotation)))
  (for _array_element _outoverlappingactors
    (Utilities|IsValid _array_element
      (:Is%20Valid
        (bind _returnvalue_2 (Class|BlueprintFunctionLibraryBase|IsFriends _array_element (Ability|GetAvatarActorfromActorInfo)))
        (if (not _returnvalue_2)
          (Class|DamageGameplayAbilityBase|CauseDamage _array_element))))))