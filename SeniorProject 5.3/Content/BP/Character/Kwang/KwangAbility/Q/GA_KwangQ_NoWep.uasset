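; GA_KwangQ_NoWep is a gameplay ability for the Kwang character that catches the sword back when it is not in hand.
; On activation it commits to casting and ends at once if the weapon is already active.
; Otherwise the server destroys the sword, the catch montage plays, and a Montage.Kwang gameplay event makes the server set the weapon active.
; The ability ends when the montage completes, blends out or is interrupted.
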(event Ability|EventActivateAbility
  (bind _returnvalue (Ability|GetAvatarActorfromActorInfo))
  (Class|GameplayAbilityBase|ActivateCasting)
  (Utilities|IsValid _returnvalue
    (:Is%20Valid
      (bind _askwang_player (Utilities|Casting|CastToKwangPlayer _returnvalue))
      (Utilities|IsValid _askwang_player
        (:Is%20Valid
          (bind _output_get (Variables|Default|SetKwang _askwang_player))
          (bind _returnvalue_2 (Class|KwangPlayer|GetbActiveWep _output_get))
          (if _returnvalue_2
            (Ability|EndAbility :!label _label)
            (else
              (Ability|HasAuthority
                (:True
                  (Class|KwangPlayer|DestroySword (Variables|Default|GetKwang)))
                (:False
                  _))
              (|PlayMontageandWaitProxy "None" "/Game/BP/Character/Kwang/Animation/Ability_Q_Catch_Montage.Ability_Q_Catch_Montage" 1.0 "None" false 1.0 0.0 false
                (:then
                  (Ability|Tasks|WaitGameplayEvent "(TagName=\"Montage.Kwang\")" 0
                    (:then
                      (Ability|HasAuthority
                        (:True
                          (Class|KwangPlayer|SetbActiveWep (Variables|Default|GetKwang) true))))))
                (:OnCompleted
                  (Ability|EndAbility :!label _label_2))
                (:OnBlendOut
                  (goto _label_2))
                (:OnInterrupted
                  (goto _label_2))
                (:OnCancelled
                  (goto _label_2))))))
        (:Is%20Not%20Valid
          (goto _label))))
    (:Is%20Not%20Valid
      (goto _label))))

(event Ability|EventOnEndAbility
  (params (bWasCancelled :type Boolean)))