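; Sword actor for Kwang's Q ability, owned by the Kwang player and destroyed if it has no owner.
; On BeginPlay it binds to the player's sword-destroy delegate, then after short delays plays the Q end sound and unbinds the sphere's begin-overlap events.
; The delegate destroys the sword after a brief delay.
; FollowingOwnerActor, not called within this Blueprint, steps the sword toward Kwang at a fixed rate scaled by its input.
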(event OnComponentBeginOverlap(Mesh)
  (params (OverlappedComponent :type Primitive%20Component%20Object%20Reference) (OtherActor :type Actor%20Object%20Reference) (OtherComp :type Primitive%20Component%20Object%20Reference) (OtherBodyIndex :type Integer) (bFromSweep :type Boolean) (SweepResult :type Hit%20Result%20Structure%20%28by%20ref%29)))

(event Custom|SwordDestroyDelegate_이벤트
  (Utilities|FlowControl|Delay 0.1)
  (Actor|DestroyActor))

(event EventBeginPlay
  (bind _returnvalue (Class|ProjectileBase|GetOwnerActor))
  (Utilities|IsValid _returnvalue
    (:Is%20Valid
      (bind _askwang_player (Utilities|Casting|CastToKwangPlayer _returnvalue))
      (bind _output_get (Variables|Default|SetKwang _askwang_player))
      (EventDispatchers|AssignSwordDestroyDelegate _output_get (delegate Custom|SwordDestroyDelegate_이벤트))
      (Utilities|FlowControl|Delay 0.4)
      (Audio|PlaySoundatLocation "/Game/Sound/Kwang_Ability_Q_End_Cue.Kwang_Ability_Q_End_Cue" (Transformation|GetActorLocation) "0, 0, 0" 1.0 1.0 0.0 0 0 0 0)
      (Utilities|FlowControl|Delay 0.3)
      (EventDispatchers|UnbindallEventsfromOnComponentBeginOverlap (Variables|Default|GetSphereComponent)))
    (:Is%20Not%20Valid
      (Actor|DestroyActor))))

(fn ConstructionScript)

(fn FollowingOwnerActor
  (params (A :type Float%20%28single-precision%29))
  (Transformation|SetActorLocation (+ (* A (* (Math|Vector|Normalize (- (Transformation|GetActorLocation (Variables|Default|GetKwang)) (Transformation|GetActorLocation))) (Math|Float|MakeLiteralFloat 5e+03))) (Transformation|GetActorLocation)) false false))