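; Gameplay ability for ranged minions that fires a projectile at the avatar's current combat target.
; With a valid target, it plays the attack montage, waits for the RangeAttack gameplay event, then spawns the projectile from the weapon socket toward the target's location.
; A following ResetCombo event, or montage completion or cancellation after a short delay, broadcasts attack end through the custom ability system component and ends the ability.
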(event Ability|EventActivateAbility
  (bind _returnvalue (Class|EnemyInterface|GetCombatTarget(Message) (Ability|GetAvatarActorfromActorInfo)))
  (bind _output_get (Variables|Default|SetTargetActor _returnvalue))
  (Utilities|IsValid _output_get
    (:Is%20Valid
      (|PlayMontageandWaitProxy "None" "/Game/BP/Character/Minion/Ranged/Animation/Range_Attack_Montage.Range_Attack_Montage" 1.0 "None" true 1.0 0.0 false
        (:then
          (Ability|Tasks|WaitGameplayEvent "(TagName=\"Abilities.Combat.RangeAttack\")" 0
            (:EventReceived
              (Class|ProjectileSpellBase|SpawnProjectile (Transformation|GetActorLocation (Variables|Default|GetTargetActor)) (GameplayTags|MakeLiteralGameplayTag "(TagName=\"CombatSocket.Weapon\")") false 0.0)
              (Ability|Tasks|WaitGameplayEvent "(TagName=\"Abilities.Combat.ResetCombo\")" 0
                (:EventReceived
                  _)))))
        (:OnCompleted
          (Utilities|FlowControl|Delay 0.5 :!label _label))
        (:OnCancelled
          (goto _label)))
      (CallFunction|BroadCastAttackEnd)
      (Ability|EndAbility))))

(event Ability|EventOnEndAbility
  (params (bWasCancelled :type Boolean)))

(fn BroadCastAttackEnd
  (bind _asability_system_component_base (Utilities|Casting|CastToAbilitySystemComponentBase (Ability|GetAbilitySystemComponent (Ability|GetAvatarActorfromActorInfo))))
  (Class|AbilitySystemComponentBase|BroadCastAttackEnd _asability_system_component_base))