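; Gameplay ability for the siege minion's ranged attack against its current combat target.
; On activation it gets the target and attack montage from the avatar through combat messages, then plays the montage.
; A RangeAttack gameplay event spawns a projectile from the weapon socket toward the target's location.
; A following ResetCombo event, or montage completion or cancellation after a short delay, broadcasts attack end on the ability system component and ends the ability.
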(event Ability|EventActivateAbility
  (bind _returnvalue (Ability|GetAvatarActorfromActorInfo))
  (Utilities|IsValid _returnvalue
    (:Is%20Valid
      (bind _output_get (Variables|Default|SetControlledPawn _returnvalue))
      (bind _returnvalue_2 (Class|EnemyInterface|GetCombatTarget(Message) _output_get))
      (bind _output_get_2 (Variables|Default|SetTargetActor _returnvalue_2))
      (Utilities|IsValid _output_get_2
        (:Is%20Valid
          (bind _returnvalue_3 (Class|CombatInterface|GetAttackMontage(Message) (Variables|Default|GetControlledPawn)))
          (|PlayMontageandWaitProxy "None" _returnvalue_3 1.0 "None" true 1.0 0.0 false
            (:then
              (Ability|Tasks|WaitGameplayEvent "(TagName=\"Abilities.Combat.RangeAttack\")" 0
                (:EventReceived
                  (Class|ProjectileSpellBase|SpawnProjectile (Transformation|GetActorLocation (Variables|Default|GetTargetActor)) (GameplayTags|MakeLiteralGameplayTag "(TagName=\"CombatSocket.Weapon\")") false 0.0)
                  (Ability|Tasks|WaitGameplayEvent "(TagName=\"Abilities.Combat.ResetCombo\")" 0
                    (:EventReceived
                      _)))))
            (:OnCompleted
              (Utilities|FlowControl|Delay 0.5 :!label _label))
            (:OnCancelled
              (goto _label)))
          (CallFunction|BroadCastAttackEnd)
          (Ability|EndAbility))))))

(event Ability|EventOnEndAbility
  (params (bWasCancelled :type Boolean)))

(fn BroadCastAttackEnd
  (bind _asability_system_component_base (Utilities|Casting|CastToAbilitySystemComponentBase (Ability|GetAbilitySystemComponent (Ability|GetAvatarActorfromActorInfo))))
  (Class|AbilitySystemComponentBase|BroadCastAttackEnd _asability_system_component_base))