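; Gameplay Ability that plays a death reaction on the avatar character.
; On activation it applies GE_HitReact to the owner and gets the death animation through CombatInterface.
; It overrides the mesh's animation data to play that asset once, without a montage.
; It then immediately removes the effect and ends, without waiting for the animation to finish.
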(event Ability|EventActivateAbility
  (bind _output_get (Variables|Default|SetAvatarActor (Ability|GetAvatarActorfromActorInfo)))
  (Utilities|IsValid _output_get
    (:Is%20Valid
      (bind _returnvalue (Ability|ApplyGameplayEffectToOwner "/Game/BP/AbilitySystem/CommonAbility/CommonAbility/GE_HitReact.GE_HitReact_C"))
      (Variables|Default|SetGE_DieReact _returnvalue)
      (bind _as캐릭터 (Utilities|Casting|CastToCharacter (Variables|Default|GetAvatarActor)))
      (Utilities|IsValid _as캐릭터
        (:Is%20Valid
          (bind _ascombat_interface (Utilities|Casting|CastToCombatInterface (Variables|Default|GetAvatarActor)))
          (bind _returnvalue_2 (Class|CombatInterface|GetDieAnimationAsset _ascombat_interface))
          (Components|Animation|OverrideAnimationData (Variables|/Script/Engine.Character|GetMesh _as캐릭터) _returnvalue_2 false true 0.0 1.0)
          (Ability|RemoveGameplayEffectFromOwnerWithHandle (Variables|Default|GetGE_DieReact))
          (Ability|EndAbility))))))

(event Ability|EventOnEndAbility
  (params (bWasCancelled :type Boolean)))