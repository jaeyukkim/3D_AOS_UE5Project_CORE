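; Gameplay ability for the Kwang player's melee attack, which runs only while the weapon is active.
; It plays the avatar's attack montage, and a MeleeAttack gameplay event triggers a sphere check in front that damages living non-friendly players.
; SaveCombo, ResetCombo or montage outcomes end the ability, some after a delay.
; AttackSpeed drives montage rate and an exponentially shrinking delay; the knockback impulse is disconnected.
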(event Ability|EventActivateAbility
  (bind _returnvalue (Ability|GetAvatarActorfromActorInfo))
  (bind _returnvalue_2 (Ability|GetAvatarActorfromActorInfo))
  (Utilities|IsValid _returnvalue_2
    (:Is%20Valid
      (bind _askwang_player (Utilities|Casting|CastToKwangPlayer _returnvalue_2))
      (Utilities|IsValid _askwang_player
        (:Is%20Valid
          (bind _output_get (Variables|Default|SetKwang _askwang_player))
          (bind _returnvalue_3 (Class|KwangPlayer|GetbActiveWep _output_get))
          (if _returnvalue_3
            (bind _ascombat_interface (Utilities|Casting|CastToCombatInterface (Ability|GetAvatarActorfromActorInfo)))
            (bind _returnvalue_4 (Class|CombatInterface|GetAttackMontage _ascombat_interface))
            (bind _outattackrate (CallFunction|CalcAttackMontageSpeed))
            (|PlayMontageandWaitProxy "None" _returnvalue_4 _outattackrate "None" true 1.0 0.0 false
              (:then
                (Ability|Tasks|WaitGameplayEvent "(TagName=\"Abilities.Combat.MeleeAttack\")" 0
                  (:then
                    (Ability|Tasks|WaitGameplayEvent "(TagName=\"Abilities.Combat.SaveCombo\")" 0
                      (:EventReceived
                        (bind _outattackdelayrate (CallFunction|CalcAttackDelayRate))
                        (Utilities|FlowControl|Delay _outattackdelayrate)
                        (Ability|EndAbility :!label _label))))
                  (:EventReceived
                    (bind _location (CallFunction|GetAttackLocation))
                    (bind _outoverlappingactors (Class|BlueprintFunctionLibraryBase|GetLivePlayersWithinRadius _returnvalue (Utilities|Array|MakeArray _returnvalue) 1e+02 _location))
                    (for _array_element _outoverlappingactors
                      (bind _returnvalue_5 (Class|BlueprintFunctionLibraryBase|IsFriends _array_element (Ability|GetAvatarActorfromActorInfo)))
                      (if _returnvalue_5
                        _
                        (else
                          (CallFunction|DamageandNcockBack _array_element)))
                      (Ability|Tasks|WaitGameplayEvent "(TagName=\"Abilities.Combat.ResetCombo\")" 0
                        (:EventReceived
                          (goto _label)))))))
              (:OnCompleted
                (goto _label))
              (:OnBlendOut
                (goto _label))
              (:OnInterrupted
                (bind _outattackdelayrate_2 (CallFunction|CalcAttackDelayRate :!label _label_2))
                (Utilities|FlowControl|Delay _outattackdelayrate_2)
                (goto _label))
              (:OnCancelled
                (goto _label_2)))
            (else
              (Ability|EndAbility))))))))

(event Ability|EventOnEndAbility
  (params (bWasCancelled :type Boolean)))

(fn GetAttackLocation
  (bind _returnvalue (Ability|GetAvatarActorfromActorInfo))
  (return (+ (Transformation|GetActorLocation _returnvalue) (* (Transformation|GetActorForwardVector _returnvalue) "125.000000,125.000000,125.000000"))))

(fn DamageandNcockBack
  (params (TargetActor :type Actor%20Object%20Reference))
  (Class|DamageGameplayAbilityBase|CauseDamage TargetActor))

(fn CalcAttackMontageSpeed
  (bind _returnvalue (GameplayAttributes|GetAttributeSet (Ability|GetAbilitySystemComponent (Ability|GetAvatarActorfromActorInfo)) "/Script/GameplayAbilities.AttributeSet"))
  (bind _asattribute_set_base (Utilities|Casting|CastToAttributeSetBase _returnvalue)
    (:then
      (return (- (Variables|Default|GetBaseDelayRate) (Math|Float|SafeDivide 1.0 (.CurrentValue (Utilities|Struct|BreakGameplayAttributeData (Variables|/Script/SeniorProject.AttributeSetBase|GetAttackSpeed _asattribute_set_base)))))))
    (:CastFailed
      (return 1.0))))

(fn CalcAttackDelayRate
  (bind _returnvalue (GameplayAttributes|GetAttributeSet (Ability|GetAbilitySystemComponent (Ability|GetAvatarActorfromActorInfo)) "/Script/GameplayAbilities.AttributeSet"))
  (bind _asattribute_set_base (Utilities|Casting|CastToAttributeSetBase _returnvalue)
    (:then
      (return (Class|KismetMathLibrary|Exp (* -1.9 (- (.CurrentValue (Utilities|Struct|BreakGameplayAttributeData (Variables|/Script/SeniorProject.AttributeSetBase|GetAttackSpeed _asattribute_set_base))) 1.0)))))
    (:CastFailed
      (return 1.0))))