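; Melee attack ability that plays the avatar's attack montage against its current combat target, both fetched through avatar messages.
; A MeleeAttack gameplay event damages the target unless it is friendly; the knockback impulse is disconnected.
; A following SaveCombo event, or montage completion or blend-out, broadcasts attack end through the ASC and ends the ability.
; Interruption or cancellation does so after a delay, while an invalid target never reaches EndAbility.
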(event Ability|EventActivateAbility
  (bind _returnvalue (Class|EnemyInterface|GetCombatTarget(Message) (Ability|GetAvatarActorfromActorInfo)))
  (bind _output_get (Variables|Default|SetTagetActor _returnvalue))
  (Utilities|IsValid _output_get
    (:Is%20Valid
      (bind _returnvalue_2 (Class|CombatInterface|GetAttackMontage(Message) (Ability|GetAvatarActorfromActorInfo)))
      (|PlayMontageandWaitProxy "None" _returnvalue_2 1.0 "None" true 1.0 0.0 false
        (:then
          (Ability|Tasks|WaitGameplayEvent "(TagName=\"Abilities.Combat.MeleeAttack\")" 0
            (:EventReceived
              (bind _returnvalue_3 (Class|BlueprintFunctionLibraryBase|IsFriends (Variables|Default|GetTagetActor) (Ability|GetAvatarActorfromActorInfo)))
              (if _returnvalue_3
                _
                (else
                  (CallFunction|DamageandNcockBack (Variables|Default|GetTagetActor))))
              (Ability|Tasks|WaitGameplayEvent "(TagName=\"Abilities.Combat.SaveCombo\")" 0
                (:EventReceived
                  _)))))
        (:OnCompleted
          _)
        (:OnBlendOut
          _)
        (:OnInterrupted
          (Utilities|FlowControl|Delay 1.0 :!label _label))
        (:OnCancelled
          (goto _label)))
      (CallFunction|BroadCastAttackEnd)
      (Ability|EndAbility))))

(event Ability|EventOnEndAbility
  (params (bWasCancelled :type Boolean)))

(fn GetAttackLocation
  (bind _returnvalue (Ability|GetAvatarActorfromActorInfo))
  (return (+ (Transformation|GetActorLocation _returnvalue) (* (Transformation|GetActorForwardVector _returnvalue) "125.000000,125.000000,125.000000"))))

(fn DamageandNcockBack
  (params (TargetActor :type Actor%20Object%20Reference))
  (Class|DamageGameplayAbilityBase|CauseDamage TargetActor))

(fn BroadCastAttackEnd
  (bind _asability_system_component_base (Utilities|Casting|CastToAbilitySystemComponentBase (Ability|GetAbilitySystemComponent (Ability|GetAvatarActorfromActorInfo)))
    (:then
      (Class|AbilitySystemComponentBase|BroadCastAttackEnd _asability_system_component_base))
    (:CastFailed
      _))
  (return))