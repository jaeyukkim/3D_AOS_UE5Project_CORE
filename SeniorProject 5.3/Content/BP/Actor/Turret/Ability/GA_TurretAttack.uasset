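; Gameplay Ability for the turret's ranged attack on the combat target reported by its avatar actor.
; It plays the attack montage, waits for the RangeAttack gameplay event, then spawns a projectile from the weapon socket toward the target's location.
; After a delay, it broadcasts attack end through the custom ability system component and ends.
; Invalid targets and montage blend-out, interruption or cancellation also reach that delayed finish.
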(event Ability|EventActivateAbility
  (bind _returnvalue (Class|EnemyInterface|GetCombatTarget(Message) (Ability|GetAvatarActorfromActorInfo)))
  (bind _output_get (Variables|Default|SetTargetActor _returnvalue))
  (Utilities|IsValid _output_get
    (:Is%20Valid
      (|PlayMontageandWaitProxy "None" "/Game/BP/Actor/Turret/Animation/TurretAttack_Montage.TurretAttack_Montage" 1.0 "None" true 1.0 0.0 false
        (:then
          (Ability|Tasks|WaitGameplayEvent "(TagName=\"Abilities.Combat.RangeAttack\")" 0
            (:EventReceived
              (Class|ProjectileSpellBase|SpawnProjectile (Transformation|GetActorLocation (Variables|Default|GetTargetActor)) (GameplayTags|MakeLiteralGameplayTag "(TagName=\"CombatSocket.Weapon\")") false 0.0)
              (Utilities|FlowControl|Delay 1.3 :!label _label))))
        (:OnBlendOut
          (Utilities|FlowControl|Delay 1.9 :!label _label_2))
        (:OnInterrupted
          (goto _label_2))
        (:OnCancelled
          (goto _label_2))))
    (:Is%20Not%20Valid
      (goto _label)))
  (CallFunction|BroadCastAttackEnd)
  (Ability|EndAbility))

(event Ability|EventOnEndAbility
  (params (bWasCancelled :type Boolean)))

(fn BroadCastAttackEnd
  (bind _asability_system_component_base (Utilities|Casting|CastToAbilitySystemComponentBase (Ability|GetAbilitySystemComponent (Ability|GetAvatarActorfromActorInfo))))
  (Class|AbilitySystemComponentBase|BroadCastAttackEnd _asability_system_component_base))