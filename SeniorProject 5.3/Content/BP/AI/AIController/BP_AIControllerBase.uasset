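; Base AI controller that points lane minions at the enemy turret they should attack next.
; On the server it binds to the game mode's minion-target update and also runs an initial refresh after a short delay.
; Each refresh gets the valid turret tier for the minion's team and lane, then scans all turrets and writes matches to the TargetTurret blackboard key.
; For the Nexus tier, any enemy turret qualifies, regardless of lane or level.
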(event Custom|UpdateMinionTargets_이벤트
  (CallFunction|UpdateTargetTurret))

(event EventBeginPlay
  (Networking|SwitchHasAuthority
    (:Authority
      (bind _asmy_game_mode_base (Utilities|Casting|CastToMyGameModeBase (Game|GetGameMode)))
      (Utilities|IsValid _asmy_game_mode_base
        (:Is%20Valid
          (bind _output_get (Variables|Default|SetGameMode _asmy_game_mode_base))
          (EventDispatchers|AssignUpdateMinionTargets _output_get (delegate Custom|UpdateMinionTargets_이벤트))
          (Utilities|FlowControl|Delay 3.0)
          (CallFunction|UpdateTargetTurret))))))

(event EventTick
  (params (DeltaSeconds :type Float%20%28single-precision%29)))

(fn ConstructionScript)

(fn UpdateTargetTurret
  (bind _returnvalue (Pawn|GetControlledPawn))
  (bind _gamemode (Variables|Default|GetGameMode))
  (Utilities|IsValid _returnvalue
    (:Is%20Valid
      (Variables|Default|SetControlledPawn _returnvalue)
      (bind _returnvalue_2 (Class|GameRuleInterface|GetLineTag(Message) (Variables|Default|GetControlledPawn)))
      (Variables|Default|SetMinionLineTag _returnvalue_2)
      (bind _returnvalue_3 (Class|GameRuleInterface|GetTeamName(Message) (Variables|Default|GetControlledPawn)))
      (Variables|Default|SetMinionTeamName _returnvalue_3)
      (Utilities|IsValid _gamemode
        (:Is%20Valid
          (bind _returnvalue_4 (Class|MyGameModeBase|GetValidTargetTurret _gamemode (Variables|Default|GetMinionTeamName) (Variables|Default|GetMinionLineTag)))
          (Variables|Default|SetNewTerretTag _returnvalue_4)
          (bind _outactors (Actor|GetAllActorsOfClass "/Script/SeniorProject.Turret"))
          (for _array_element _outactors
            (bind _output_get (Variables|Default|SetNewTurret _array_element))
            (Utilities|IsValid _output_get
              (:Is%20Valid
                (bind _returnvalue_5 (Class|GameRuleInterface|GetTurretLevelTag(Message) (Variables|Default|GetNewTurret)))
                (bind _returnvalue_6 (Class|GameRuleInterface|GetTeamName(Message) (Variables|Default|GetNewTurret)))
                (bind _returnvalue_7 (Class|GameRuleInterface|GetLineTag(Message) (Variables|Default|GetNewTurret)))
                (if (Math|Boolean|ANDBoolean (!= _returnvalue_6 (Variables|Default|GetMinionTeamName)) (== _returnvalue_5 (Variables|Default|GetNewTerretTag)) (== _returnvalue_7 (Variables|Default|GetMinionLineTag)))
                  (AI|Components|Blackboard|SetValueasObject (AI|GetBlackboard 0) (Variables|Default|GetTargetTurret) (Variables|Default|GetNewTurret) :!label _label)
                  (elif (and (== "(TagName=\"GameRule.Turret.Nexus\")" (Variables|Default|GetNewTerretTag)) (!= (Variables|Default|GetMinionTeamName) _returnvalue_6))
                    (goto _label)))))))))))